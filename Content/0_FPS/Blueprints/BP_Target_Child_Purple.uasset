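; BP_Target_Child_Purple is the purple child variant of an FPS target that moves back and forth along a line.
; Each Tick offsets the actor along the normalized DirectionPurple1 by SpeedPurple, without sweep or delta-time scaling, so speed depends on frame rate.
; A looping timer started on BeginPlay negates that direction every MovementDurationPurple1 seconds.
; The construction script only calls its parent.
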(event Custom|CustomEvent
  ;[0.008421 0.15 0.000469 0.5] Turn One
  (Variables|Default|SetDirection%20Purple%201 (* (Variables|Default|GetDirection%20Purple%201) -1.0)))

(event EventBeginPlay
  ;[0.008421 0.15 0.000469 0.5] Turn One
  (Utilities|Time|SetTimerbyEvent (delegate Custom|CustomEvent) (Variables|Default|GetMovement%20Duration%20Purple%201) true))

(event EventTick
  (params (DeltaSeconds :type Float%20%28single-precision%29))
  ;[0.15 0 0.03222 0.5] Target Movement
  (Transformation|AddActorWorldOffset (* (Math|Vector|Normalize (Variables|Default|GetDirection%20Purple%201)) (Variables|Default|GetSpeed%20Purple))))

(fn ConstructionScript
  (|CallParentFunction))