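; Security camera that sweeps back and forth and catches the player when its line of sight hits them.
; MoveCamera loops by calling itself, using a FlipFlop to alternate start and end rotations with timed interpolation and a delay.
; Each Tick, a debug-drawn Pawn object trace runs forward from the LineTrace component.
; Hitting the player sets IsCaught on BP_FirstPersonCharacter, disables its input and prints a message.
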(event Custom|MoveCamera
  ;[0.15 0.15 0.15 0.5] Move Camera
  (Utilities|FlowControl|FlipFlop
    (:A
      (Variables|Default|SetCurrentRotation (Variables|Default|GetEndRotation)))
    (:B
      (Variables|Default|SetCurrentRotation (Variables|Default|GetStartRotation))))
  (Components|MoveComponentTo (Variables|Default|GetSM_Camera) "0, 0, 0" (Variables|Default|GetCurrentRotation) false false (Variables|Default|GetSpeed) false)
  (Utilities|FlowControl|Delay (Variables|Default|GetDelay))
  (CallFunction|MoveCamera))

(event Custom|Detect
  (bind _linetrace (Variables|Default|GetLineTrace))
  (bind _returnvalue (Transformation|GetWorldLocation _linetrace))
  ;[0.15 0.15 0.15 0.5] Detect Player
  (bind _outhit (Collision|LineTraceForObjects _returnvalue (+ _returnvalue (* (Math|Vector|GetForwardVector (Transformation|GetWorldRotation _linetrace)) (Variables|Default|GetDetectDistance))) (Utilities|Array|MakeArray "ObjectTypeQuery3") false 0 "ForOneFrame"))
  (if (== (.HitActor (Collision|BreakHitResult _outhit)) (Variables|Default|GetPlayerReference))
    (Utilities|FlowControl|Sequence
      (:then_0
        (Variables|/Game/0_FPS/Blueprints/BP_FirstPersonCharacter.BP_FirstPersonCharacter_C|SetIsCaught (Variables|Default|GetPlayerReference) true)
        ;[0.15 0.15 0.15 0.5] Disable Input
        (Input|DisableInput (Variables|Default|GetPlayerReference) (Game|GetPlayerController 0)))
      (:then_1
        (Development|PrintString "Caught")))))

(event EventBeginPlay
  (Utilities|FlowControl|Sequence
    (:then_0
      ;[0.15 0.15 0.15 0.5] Setup Variables
      (bind _asbp_first_person_character (Utilities|Casting|CastToBP_FirstPersonCharacter (Game|GetPlayerCharacter 0)))
      (Variables|Default|SetPlayerReference _asbp_first_person_character))
    (:then_1
      ;[0.15 0.15 0.15 0.5] Call Move Camera
      (CallFunction|MoveCamera))))

(event EventTick
  (params (DeltaSeconds :type Float%20%28single-precision%29))
  (CallFunction|Detect))

(fn ConstructionScript)