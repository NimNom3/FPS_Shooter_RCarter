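; Key-locked door actor with an indicator light that reacts when the first-person player enters its trigger zone.
; BeginPlay caches the player and puts a dynamic instance of MI_Light on the light mesh.
; On overlap the light brightens, turning green and swinging the door open via a Timeline rotation lerp if the player has the key, otherwise turning red.
; Leaving resets the light and reverses the Timeline.
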(event OnComponentBeginOverlap(DoorTriggerZone)
  (params (OverlappedComponent :type Primitive%20Component%20Object%20Reference) (OtherActor :type Actor%20Object%20Reference) (OtherComp :type Primitive%20Component%20Object%20Reference) (OtherBodyIndex :type Integer) (bFromSweep :type Boolean) (SweepResult :type Hit%20Result%20Structure%20%28by%20ref%29))
  ;[0.15 0.15 0.15 0.5] Light Change
  (if (== OtherActor (Variables|Default|GetPlayerReference))
    (Rendering|Material|SetScalarParameterValue (Variables|Default|GetDynamic%20Material) "Brightness" 1e+02 :!class /Script/Engine.MaterialInstanceDynamic)
    (if (Variables|/Game/0_FPS/Blueprints/BP_FirstPersonCharacter.BP_FirstPersonCharacter_C|GetHasKey (Variables|Default|GetPlayerReference))
      (Rendering|Material|SetVectorParameterValue (Variables|Default|GetDynamic%20Material) "Colour" "(R=0.099367,G=1.000000,B=0.000000,A=1.000000)" :!class /Script/Engine.MaterialInstanceDynamic)
      ;[0.15 0.15 0.15 0.5] Door Open Close
      (bind _alpha (Timeline|Timeline_Door_Open_Close Play)
        (:Update
          (Variables|Default|SetDoorOpening true)
          (Transformation|SetRelativeRotation (Variables|Default|GetSM_Door) (Math|Rotator|Lerp(Rotator) "0, 0, 0" "0.000000,90.000000,0.000000" _alpha) false false))
        (:Finished
          (Variables|Default|SetDoorOpening false)))
      (else
        (Rendering|Material|SetVectorParameterValue (Variables|Default|GetDynamic%20Material) "Colour" "(R=1.000000,G=0.000000,B=0.003115,A=1.000000)" :!class /Script/Engine.MaterialInstanceDynamic)))))

(event OnComponentEndOverlap(DoorTriggerZone)
  (params (OverlappedComponent :type Primitive%20Component%20Object%20Reference) (OtherActor :type Actor%20Object%20Reference) (OtherComp :type Primitive%20Component%20Object%20Reference) (OtherBodyIndex :type Integer))
  (bind _dynamic_material (Variables|Default|GetDynamic%20Material))
  ;[0.15 0.15 0.15 0.5] Reset To Default
  (if (== OtherActor (Variables|Default|GetPlayerReference))
    (Rendering|Material|SetScalarParameterValue _dynamic_material "Brightness" 1.0 :!class /Script/Engine.MaterialInstanceDynamic)
    (Rendering|Material|SetVectorParameterValue _dynamic_material "Colour" "(R=0.989601,G=1.000000,B=0.825810,A=1.000000)" :!class /Script/Engine.MaterialInstanceDynamic)
    ;[0.15 0.15 0.15 0.5] Door Open Close
    (bind _alpha (Timeline|Timeline_Door_Open_Close Reverse)
      (:Update
        (Variables|Default|SetDoorOpening true)
        (Transformation|SetRelativeRotation (Variables|Default|GetSM_Door) (Math|Rotator|Lerp(Rotator) "0, 0, 0" "0.000000,90.000000,0.000000" _alpha) false false))
      (:Finished
        (Variables|Default|SetDoorOpening false)))))

(event EventBeginPlay
  ;[0 0.15 0.09469 0.5] Setup Variable
  (Utilities|FlowControl|Sequence
    (:then_0
      ;;[0.09868 0.15 0 0.5] Setup Player Reference
      (bind _asbp_first_person_character (Utilities|Casting|CastToBP_FirstPersonCharacter (Game|GetPlayerCharacter 0)))
      (Variables|Default|SetPlayerReference _asbp_first_person_character))
    (:then_1
      ;;[0.1121 0.15 0 0.5] Setup Material Variable
      (bind _returnvalue (Rendering|Material|CreateDynamicMaterialInstance "/Game/0_FPS/Materials/MI_Light.MI_Light" "None" "None" :!class /Script/Engine.KismetMaterialLibrary))
      (bind _output_get (Variables|Default|SetDynamic%20Material _returnvalue))
      (Rendering|Material|SetMaterial (Variables|Default|GetSM_Light) 0 _output_get))))

(fn ConstructionScript)