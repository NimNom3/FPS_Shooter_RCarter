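; BP_Target_Child_Green is a green target variant, apparently for an FPS, that animates its own scale.
; Tick adds a small fixed step to a stored scale vector and applies it to the actor, so the rate depends on frame rate.
; A looping timer set at BeginPlay periodically negates the vector itself rather than the step, mirroring the scale before it climbs again.
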(event Custom|CustomEvent
  (Variables|Default|SetScale%20Green%20Scale (* (Variables|Default|GetScale%20Green%20Scale) "-1.000000,-1.000000,-1.000000")))

(event EventBeginPlay
  (Utilities|Time|SetTimerbyEvent (delegate Custom|CustomEvent) 4.0 true)
  (|CallParentFunction))

(event EventTick
  (params (DeltaSeconds :type Float%20%28single-precision%29))
  (bind _output_get (Variables|Default|SetScale%20Green%20Scale (+ (Variables|Default|GetScale%20Green%20Scale) "0.010000,0.010000,0.010000")))
  (Transformation|SetActorScale3D _output_get))

(fn ConstructionScript
  (|CallParentFunction))