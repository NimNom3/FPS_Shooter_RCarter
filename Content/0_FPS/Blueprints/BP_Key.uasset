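; BP_Key is a key actor that appears when no BP_Target actors appear to remain in the level.
; Every Tick it queries all targets and uses a value derived from that array to toggle its visibility and collision.
; The first time the value reaches zero or below, a DoOnce spawns a particle effect and plays an appearance sound at the key.
; It also prints the value each frame.
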(event EventTick
  (params (DeltaSeconds :type Float%20%28single-precision%29))
  (bind _defaultsceneroot (Variables|Default|GetDefaultSceneRoot))
  (bind _returnvalue (Transformation|GetWorldLocation _defaultsceneroot))
  ;[0 0.02207 0.15 0.5] Key Visability
  (bind _outactors (Actor|GetAllActorsOfClass "/Game/0_FPS/Blueprints/BP_Target.BP_Target_C"))
  (bind _returnvalue_2 (Utilities|Array|Add _outactors 0))
  (Utilities|FlowControl|Sequence
    (:then_0
      (Rendering|SetVisibility (Variables|Default|GetDefaultSceneRoot) (<= _returnvalue_2 0) true)
      (Collision|SetActorEnableCollision (<= _returnvalue_2 0))
      ;[0.15 0.15 0.15 0.5] Key Spawn Effect
      (if (<= _returnvalue_2 0)
        (Utilities|FlowControl|DoOnce false
          (:Completed
            (Effects|SpawnEmitteratLocation "/Engine/Tutorial/SubEditors/TutorialAssets/TutorialParticleSystem.TutorialParticleSystem" _returnvalue)
            (Audio|PlaySoundatLocation "/Game/0_FPS/Audio/MP3_Key_Appear.MP3_Key_Appear" _returnvalue "0, 0, 0" 1.0 1.0 0.0 0 0 0 0)))))
    (:then_1
      (Development|PrintString (Utilities|String|ToString(Integer) _returnvalue_2)))))

(fn ConstructionScript)