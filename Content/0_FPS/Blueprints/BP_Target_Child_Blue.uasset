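; Blue target child Blueprint that slides in a set direction for a limited time, then stops.
; Each Tick it adds a local offset of normalized DirectionBlue times SpeedBlue, without sweep or delta-time scaling, so speed depends on frame rate.
; A timer started on BeginPlay fires after MovementDurationBlue and zeroes SpeedBlue to halt it.
; The construction script only calls the parent's.
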(event Custom|Event%20Stop
  ;[0.001654 0.15 0 0.5] Stop Movement
  (Variables|Default|SetSpeed%20Blue 0.0))

(event EventTick
  (params (DeltaSeconds :type Float%20%28single-precision%29))
  ;[0.15 0 0.01376 0.5] Movement
  (Transformation|AddActorLocalOffset (* (Math|Vector|Normalize (Variables|Default|GetDirection%20Blue)) (Variables|Default|GetSpeed%20Blue)) false false))

(event EventBeginPlay
  ;[0.001654 0.15 0 0.5] Stop Movement
  (Utilities|Time|SetTimerbyEvent (delegate Custom|Event%20Stop) (Variables|Default|GetMovement%20Duration%20Blue)))

(fn ConstructionScript
  (|CallParentFunction))